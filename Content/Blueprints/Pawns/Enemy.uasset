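; Enemy pawn that turns to face the player and fires projectiles at a steady interval.
; BeginPlay caches the first FirstPersonCharacter_BP as the target, and Tick snaps the actor's rotation toward it.
; Tick also spawns EnemyProjectile at the Arrow component through a DoOnce that resets after a short delay.
; An AI move meant to back away from the player is left unconnected and never runs.
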(event EventBeginPlay
  (bind _outactors (Actor|GetAllActorsOfClass "/Game/Blueprints/Pawns/FirstPersonCharacter_BP.FirstPersonCharacter_BP_C"))
  (Variables|Default|Settarget (Utilities|Array|Get(acopy) _outactors)))

(event Collision|EventActorBeginOverlap
  (params (OtherActor :type Actor%20Object%20Reference)))

(event EventTick
  (params (DeltaSeconds :type Float%20%28single-precision%29))
  (bind _arrow (Variables|Default|GetArrow))
  (Utilities|FlowControl|Sequence
    (:then_0
      ;[1 1 1] Rotate to player
      (Transformation|SetActorRotation (Math|Rotator|FindLookatRotation (Transformation|GetActorLocation) (Transformation|GetActorLocation (Variables|Default|Gettarget)))))
    (:then_2
      (Utilities|FlowControl|DoOnce false :!label _label
        (:Completed
          (Game|SpawnActorfromClass "/Game/Blueprints/Actors/EnemyProjectile.EnemyProjectile_C" (Math|Transform|MakeTransform (Transformation|GetWorldLocation _arrow) (Transformation|GetWorldRotation _arrow) "1,1,1") "Undefined" 0 0)
          (Utilities|FlowControl|Delay 0.5)
          (goto _label Reset))))))

(fn ConstructionScript)